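; BP_Door is a door Blueprint that swings open once it has received the required number of keys.
; AddKey increments a key counter and calls OpenDoor when the count equals KeysNeeded.
; OpenDoor stores the current rotation, then a timeline lerps the Door component to a fixed 90-degree world yaw, keeping its roll and pitch.
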(event Custom|OpenDoor
  (bind _door (Variables|Default|GetDoor))
  (bind _returnvalue (Transformation|GetWorldRotation _door))
  (Variables|Default|SetInitRotation (Transformation|GetWorldRotation (Variables|Default|GetDoor)))
  (Variables|Default|SetTargetRotation (Math|Rotator|MakeRotator (.roll _returnvalue) (.pitch _returnvalue) 9e+01))
  (bind _alfa (Timeline|DoorRatation Play)
    (:Update
      (Transformation|SetWorldRotation (Variables|Default|GetDoor) (Math|Rotator|Lerp(Rotator) (Variables|Default|GetInitRotation) (Variables|Default|GetTargetRotation) _alfa) false false))))

(event EventBeginPlay)

(event Collision|EventActorBeginOverlap
  (params (OtherActor :type Actor%20Object%20Reference)))

(event EventTick
  (params (DeltaSeconds :type Float%20%28single-precision%29)))

(fn ConstructionScript)

(fn AddKey
  (Math|Integer|IncrementInt (Variables|Default|GetCurentKeysNumber)
    (:%20%20
      (if (== (Variables|Default|GetCurentKeysNumber) (Variables|Default|GetKeysNeeded))
        (CallFunction|OpenDoor)))))