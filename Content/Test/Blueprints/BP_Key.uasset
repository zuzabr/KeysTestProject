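; BP_Key is a key actor that the player picks up through interaction if not already holding one.
; A widget shows while the key is in the player's field of view.
; On pickup, a timeline lerps the key to the mesh's KeySocket, attaching it, disabling collision and hiding the widget on each update.
; Remove detaches the key and snaps it onto a supplied component when valid.
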(event EventBeginPlay)

(event Collision|EventActorBeginOverlap
  (params (OtherActor :type Actor%20Object%20Reference)))

(event EventTick
  (params (DeltaSeconds :type Float%20%28single-precision%29)))

(event EventInFovOfPlayer
  (params (InFov :type Boolean))
  (Rendering|SetVisibility (Variables|Default|GetWidget) InFov false))

(event EventInteraction
  (params (Player :type BP%20Third%20Person%20Character%20Object%20Reference))
  ;[1 1 1] Если бы не через таймлайн, а через анимацию и notifies можно было убрать в универсальную функцию
  (if (not (.HasKey (Default|GetAttachedKey Player)))
    (Variables|Default|SetInitTransform (Transformation|GetActorTransform))
    (bind _alfa (Timeline|KeyRelocation Play)
      (:Update
        (CallFunction|AttachtoCharacter Player _alfa)))))

(event EventRemove
  (params (NewAttachComp :type Scene%20Component%20Object%20Reference))
  (Transformation|DetachFromActor "KeepRelative" "KeepRelative" "KeepRelative")
  (Utilities|IsValid NewAttachComp
    (:Is%20Valid
      (Transformation|AttachComponentToComponent NewAttachComp "None" "SnapToTarget" "SnapToTarget" "SnapToTarget" true))))

(fn ConstructionScript)

(fn AttachtoCharacter
  (params (Player :type BP%20Third%20Person%20Character%20Object%20Reference) (Alpha :type Float%20%28single-precision%29))
  (Transformation|SetActorTransform (Math|Transform|Lerp(Transform) (Variables|Default|GetInitTransform) (Transformation|GetSocketTransform (Variables|/Script/Engine.Character|GetMesh Player) "KeySocket" "RTS_World") Alpha))
  (Transformation|AttachActorToActor Player "KeySocket" "SnapToTarget" "KeepRelative" "SnapToTarget" true)
  (Collision|SetActorEnableCollision false)
  (Rendering|SetVisibility (Variables|Default|GetWidget) false false))