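; BP_Stand is an interactable key stand that takes the key a player carries and registers it with a linked door.
; Its prompt widget follows the player's field of view while the stand is usable.
; A successful interaction disables the stand, hides the widget, removes the key to PlaceForKey and calls AddKey on ConnectedDoor.
; It prints a warning if no door is assigned.
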(event EventBeginPlay)

(event Collision|EventActorBeginOverlap
  (params (OtherActor :type Actor%20Object%20Reference)))

(event EventTick
  (params (DeltaSeconds :type Float%20%28single-precision%29)))

(event EventInFovOfPlayer
  (params (InFov :type Boolean))
  (if (Variables|Default|GetCanInteract)
    (Rendering|SetVisibility (Variables|Default|GetWidget) InFov false)))

(event EventInteraction
  (params (Player :type BP%20Third%20Person%20Character%20Object%20Reference))
  (bind (_haskey _key) (Default|GetAttachedKey Player))
  (if (Variables|Default|GetCanInteract)
    (if _haskey
      (bind _output_get (Variables|Default|SetCanInteract false))
      (Rendering|SetVisibility (Variables|Default|GetWidget) _output_get false)
      (Default|Remove _key (Variables|Default|GetPlaceForKey))
      (Utilities|IsValid (Variables|Default|GetConnectedDoor)
        (:Is%20Valid
          (Default|AddKey (Variables|Default|GetConnectedDoor)))
        (:Is%20Not%20Valid
          (Development|PrintString "Forget to set the door on the stand"))))))

(fn ConstructionScript)